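; BP_PlayerPawn is the player's rolling ball pawn, moved by physics torque.
; The forward/backward and left/right axis inputs apply scaled torque to the static mesh as an acceleration change, so mass is ignored.
; BeginPlay fades the camera in, and any damage triggers a one-time fade out, short delay and reload of the current level.
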(event EventBeginPlay
  (CameraFades|StartCameraFade :self (Game|GetPlayerCameraManager 0) :FromAlpha 1.0 :Duration 2.0 :bHoldWhenFinished true))

(event Collision|EventActorBeginOverlap
  (params (OtherActor :type Actor%20Object%20Reference)))

(event EventTick
  (params (DeltaSeconds :type Float%20%28single-precision%29)))

(event Game|Damage|EventAnyDamage
  (params (Damage :type Float%20%28single-precision%29) (DamageType :type Damage%20Type%20Object%20Reference) (InstigatedBy :type Controller%20Object%20Reference) (DamageCauser :type Actor%20Object%20Reference))
  (bind _returnvalue (Math|Float|MakeLiteralFloat 0.5))
  (Utilities|FlowControl|DoOnce false
    (:Completed
      (CameraFades|StartCameraFade :self (Game|GetPlayerCameraManager 0) :ToAlpha 1.0 :Duration _returnvalue :bHoldWhenFinished true)
      (Utilities|FlowControl|Delay _returnvalue)
      (bind _returnvalue_2 (Game|GetCurrentLevelName true))
      (Game|OpenLevel(byName) (Utilities|String|StringToName _returnvalue_2)))))

(event Input|AxisEvents|InputAxisMoveForwards/Backwards
  (params (AxisValue :type Float%20%28single-precision%29))
  ;[1 1 1] Ball Move Inputs
  (Class|PrimitiveComponent|AddTorqueinRadians (Variables|Default|GetStaticMesh) (Math|Vector|MakeVector (* (stale Input|AxisEvents|InputAxisMoveLeft/Right AxisValue) (Variables|Default|GetRight/Left%20Number)) (* AxisValue (Variables|Default|GetPushNumber)) 0.0) "None" true))

(event Input|AxisEvents|InputAxisMoveLeft/Right
  (params (AxisValue :type Float%20%28single-precision%29))
  ;[1 1 1] Ball Move Inputs
  (Class|PrimitiveComponent|AddTorqueinRadians (Variables|Default|GetStaticMesh) (Math|Vector|MakeVector (* AxisValue (Variables|Default|GetRight/Left%20Number)) (* (stale Input|AxisEvents|InputAxisMoveForwards/Backwards AxisValue) (Variables|Default|GetPushNumber)) 0.0) "None" true))

(fn ConstructionScript)