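; BP_Cannon is an automatic cannon actor that fires BP_ProjectTile projectiles on a repeating cycle.
; From BeginPlay it waits for the fire-rate delay, spawns a scaled projectile at the CannonSpawnPoint transform, then plays the FireAnimation timeline.
; The timeline moves the barrel's relative location on each update, and its Cannon Fired event loops back to the delay, forming a self-sustaining fire loop.
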(event EventBeginPlay
  (Utilities|FlowControl|Delay (Variables|CannonOptions|GetCannon_Fire_Rate) :!label _label)
  (CallFunction|SpawnProjectile)
  (bind _fireanimation (Timeline|FireAnimation PlayFromStart)
    (:Update
      (CallFunction|MoveCannonBarrel _fireanimation))
    (:CannonFired
      (goto _label))))

(fn ConstructionScript)

(fn SpawnProjectile
  (bind _cannon_spawn_point (Variables|Default|GetCannon%20Spawn%20Point))
  (Game|SpawnActorfromClass "/Game/BluePrints/Actors/ProjectTiles/BP_ProjectTile.BP_ProjectTile_C" (Math|Transform|MakeTransform (Transformation|GetWorldLocation _cannon_spawn_point) (Transformation|GetWorldRotation _cannon_spawn_point) (Math|Conversions|ToVector(Float) (Variables|CannonOptions|GetProjectile_Scale))) "Undefined" 0 0))

(fn MoveCannonBarrel
  (params (NewLocation_Y :type Float%20%28single-precision%29))
  (Transformation|SetRelativeLocation (Variables|Default|GetCannon) (Math|Vector|MakeVector 0.0 NewLocation_Y 0.0) false false))